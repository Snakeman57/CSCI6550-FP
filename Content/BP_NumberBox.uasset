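; BP_NumberBox is a text entry Blueprint meant to take numeric input and store it as an integer.
; forceNum calls SetTxt, which saves numeric text in Last and reapplies it, but does not revert non-numeric text.
; storeNumber converts the given text to an integer in Num without a numeric check.
; The nodes that would bind both events to text changed and committed delegates never run.
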(event Custom|storeNumber
  (params (Text :type Text%20%28by%20ref%29) (CommitMethod :type ETextCommit%20Enum :default "Default"))
  (Variables|Default|Setnum (Math|Conversions|ToInteger(Byte) (Utilities|String|ToString(Text) Text))))

(event Custom|forceNum
  (params (Text :type Text%20%28by%20ref%29))
  (CallFunction|SetTxt Text))

(fn SetTxt
  (params (Text :type Text))
  (if (Class|KismetStringLibrary|IsNumeric (Utilities|String|ToString(Text) Text))
    (Variables|Default|Setlast Text)
    (Rendering|Components|TextRender|SetText (Variables|Default|Getlast))))